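; Actor component that runs queued dialogue, playing each entry's voice lines in sequence as Wwise events on the player pawn.
; TryQueueDialogue adds known IDs uniquely to a queue, and Tick starts the first queued dialogue whenever none is playing.
; StartDialogueData recursively waits for each audio event to finish, pauses between lines and dialogues, then clears the current entry and signals when the queue is empty.
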(event Custom|PlayDialogue
  (params (DialogueID :type String))
  (Utilities|Array|RemoveItem (Variables|Default|GetDialogueQueue) DialogueID)
  (bind _array_element (Utilities|Array|ForEachLoopwithBreak (Variables|Default|GetDialogue) :!label _label)
    (:LoopBody
      (if (Utilities|Enum|Equal(Enum) (.ID (Utilities|Struct|BreakF_DialogueData _array_element)) DialogueID)
        (Variables|Default|SetCurrentDialogueIndex 0)
        (Variables|Default|SetCurrentDialogueEntriesToPlay _array_element)
        (CallFunction|StartDialogueData)
        (goto _label Break)))))

(event Custom|StartDialogueData
  (if (< (Variables|Default|GetCurrentDialogueIndex) (Utilities|Array|Length (.dialogueentries (Variables|Default|GetCurrentDialogueEntriesToPlay))))
    (Class|AkGameplayStatics|PostandWaitforEndOfEvent (.audio (Utilities|Array|Get(acopy) (.dialogueentries (Variables|Default|GetCurrentDialogueEntriesToPlay)) (Variables|Default|GetCurrentDialogueIndex))) (Game|Player|GetPlayerPawn 0))
    (Utilities|FlowControl|Delay (Variables|Default|GetPauseBeforeNextLine))
    (Math|Integer|IncrementInt (Variables|Default|GetCurrentDialogueIndex)
      (:%20%20
        (CallFunction|StartDialogueData)))
    (else
      (Utilities|FlowControl|Delay (Variables|Default|GetPauseBeforeNextDialogueEntry))
      (Variables|Default|SetCurrentDialogueEntriesToPlay "")
      (if (Utilities|Array|IsEmpty (Variables|Default|GetDialogueQueue))
        (Default|CallOnDialogueQueueEmpty)))))

(event EventTick
  (params (DeltaSeconds :type Float%20%28single-precision%29))
  (bind _dialoguequeue (Variables|Default|GetDialogueQueue))
  (if (Utilities|Array|IsEmpty (.id (Variables|Default|GetCurrentDialogueEntriesToPlay)))
    (if (Utilities|Array|IsNotEmpty _dialoguequeue)
      (CallFunction|PlayDialogue (Utilities|Array|Get(acopy) _dialoguequeue)))))

(fn IsViableDialogue
  (params (ID :type String))
  (for _array_element (Variables|Default|GetDialogue)
    (if (Utilities|Enum|Equal(Enum) (.id _array_element) ID)
      (return true)))
  (return false))

(fn TryQueueDialogue
  (params (DialogueID :type String))
  (if (CallFunction|IsViableDialogue DialogueID)
    (bind _returnvalue (Utilities|Array|AddUnique (Variables|Default|GetDialogueQueue) DialogueID))
    (return (>= _returnvalue 0))
    (else
      (return false))))