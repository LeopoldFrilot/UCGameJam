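; BP_DialoguePlayer is a one-shot trigger that queues a dialogue by ID when the player character overlaps its box.
; The request goes to the dialogue runner component on the GameMode, and the trigger is spent even if queuing fails.
; With camera control enabled, a successful queue starts a cutscene on the player and binds to the runner's queue-empty event, which fires DialogueFinished after a configurable delay.
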(event OnComponentBeginOverlap(Box)
  (params (OverlappedComponent :type Primitive%20Component%20Object%20Reference) (OtherActor :type Actor%20Object%20Reference) (OtherComp :type Primitive%20Component%20Object%20Reference) (OtherBodyIndex :type Integer) (bFromSweep :type Boolean) (SweepResult :type Hit%20Result%20Structure%20%28by%20ref%29))
  (CallFunction|TryStartTrigger OtherActor))

(event Custom|OnDialogueDataEnded_Event
  (Utilities|FlowControl|Delay (Variables|Default|GetTimeToRegainControlAfterDialogue))
  (Default|CallDialogueFinished))

(event Custom|TryStartTrigger
  (params (OtherActor :type Actor%20Object%20Reference))
  (bind _returnvalue (Game|GetGameMode))
  (bind _asbp_game_mode (Utilities|Casting|CastToBP_GameMode _returnvalue))
  (bind _bpc_dialoguerunner (Variables|/Game/Blueprints/Core/BP_GameMode.BP_GameMode_C|GetBPC_DialogueRunner _asbp_game_mode))
  (bind _asbp_player_character (Utilities|Casting|CastToBP_PlayerCharacter OtherActor))
  (if (not (Variables|Default|GetTriggered))
    (Variables|Default|SetTriggered true)
    (bind _success_ (Default|TryQueueDialogue _bpc_dialoguerunner (Variables|Default|GetDialogue%20ID)))
    (if _success_
      (if (Variables|Default|GetShouldTakeCameraControl)
        (Default|StartCutscene _asbp_player_character self)
        (EventDispatchers|AssignOnDialogueQueueEmpty _bpc_dialoguerunner (delegate Custom|OnDialogueDataEnded_Event))))))

(fn ConstructionScript)