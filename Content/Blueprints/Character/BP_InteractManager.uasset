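; BP_InteractManager is an actor that tracks nearby interactable actors and decides which one can be used.
; Its collision component adds BPI_Interactable actors to a list on overlap, and switches them off and removes them when overlap ends.
; Each tick, it toggles interactability on only for the listed actor nearest to it, found by a distance search.
; Its Interact event passes the given Player to that closest interactable through the interface.
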(event OnComponentBeginOverlap(CollisionComponent)
  (params (OverlappedComponent :type Primitive%20Component%20Object%20Reference) (OtherActor :type Actor%20Object%20Reference) (OtherComp :type Primitive%20Component%20Object%20Reference) (OtherBodyIndex :type Integer) (bFromSweep :type Boolean) (SweepResult :type Hit%20Result%20Structure%20%28by%20ref%29))
  (Utilities|Casting|CastToBPI_Interactable OtherActor)
  (Utilities|Array|AddUnique (Variables|Default|GetInteractables) OtherActor))

(event OnComponentEndOverlap(CollisionComponent)
  (params (OverlappedComponent :type Primitive%20Component%20Object%20Reference) (OtherActor :type Actor%20Object%20Reference) (OtherComp :type Primitive%20Component%20Object%20Reference) (OtherBodyIndex :type Integer))
  (bind _asbpi_interactable (Utilities|Casting|CastToBPI_Interactable OtherActor))
  (Default|ToggleInteractabilityonOff _asbpi_interactable false)
  (Utilities|Array|RemoveItem (Variables|Default|GetInteractables) OtherActor))

(event Custom|Interact
  (params (Player :type BP%20Player%20Character%20Object%20Reference))
  (bind _result (CallFunction|GetClosestInteractable))
  (Utilities|IsValid _result
    (:Is%20Valid
      (bind _asbpi_interactable (Utilities|Casting|CastToBPI_Interactable _result))
      (Default|Interact _asbpi_interactable Player))))

(event EventTick
  (params (DeltaSeconds :type Float%20%28single-precision%29))
  (bind _result (CallFunction|GetClosestInteractable))
  (Utilities|IsValid _result
    (:Is%20Valid
      (for _array_element (Variables|Default|GetInteractables)
        (bind _asbpi_interactable (Utilities|Casting|CastToBPI_Interactable _array_element))
        (Default|ToggleInteractabilityonOff _asbpi_interactable (== _array_element _result))))))

(fn ConstructionScript)

(fn GetClosestInteractable
  (for _array_element (Variables|Default|GetInteractables)
    (Utilities|IsValid _array_element
      (:Is%20Valid
        (if (< (Math|Vector|Distance(Vector) (Transformation|GetActorLocation) (Transformation|GetActorLocation _array_element)) (LocalVariables|GetSmallestDistance))
          (LocalVariables|SetSmallestDistance (Math|Vector|Distance(Vector) (Transformation|GetActorLocation) (Transformation|GetActorLocation _array_element)))
          (LocalVariables|SetReturnValue _array_element)))))
  (return (LocalVariables|GetReturnValue)))