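; Character component that manages a set of unlockable abilities and lets its owner switch between them.
; Switching requires the ability to be unlocked and a shared switching cooldown to have elapsed.
; Each switch ends the current ability, then spawns the new ability class as an actor attached to the owner and activates it.
; Tick forwards a passive update to the active ability actor every frame.
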(event Custom|SwitchToAbility
  (params (AbilityIndex :type BP%20Tangram%20Ability%20Base%20Class%20Reference))
  (if (and (CallFunction|IsOffCooldown) (Utilities|Array|ContainsItem (Variables|Default|GetUnlockedAbilities) AbilityIndex))
    (bind _output_get (Variables|Default|SetCurrentActiveAbility AbilityIndex))
    (Utilities|FlowControl|Sequence
      (:then_0
        (bind _spawnedability (Variables|Default|GetSpawnedAbility)
          (:then
            (Default|EndAbility _spawnedability))
          (:else)))
      (:then_1
        (bind _returnvalue (Game|SpawnActorfromClass _output_get (Math|Transform|MakeTransform "0, 0, 0") "Undefined" "MultiplyWithRoot" (Components|GetOwner) 0))
        (bind _output_get_2 (Variables|Default|SetSpawnedAbility _returnvalue))
        (Transformation|AttachActorToActor _output_get_2 (Components|GetOwner) "None" "SnapToTarget" "KeepRelative" "KeepRelative" true)
        (Default|Activate _output_get_2)
        (Variables|Default|SetLastTimeActivated (Utilities|Time|GetGameTimeinSeconds))))))

(event Custom|UnlockAbility
  (params (Ability :type BP%20Tangram%20Ability%20Base%20Class%20Reference))
  (Utilities|Array|AddUnique (Variables|Default|GetUnlockedAbilities) Ability))

(event EventTick
  (params (DeltaSeconds :type Float%20%28single-precision%29))
  (bind _spawnedability (Variables|Default|GetSpawnedAbility)
    (:then
      (Default|UpdatePassive _spawnedability))
    (:else)))

(fn IsOffCooldown
  (return (> (Utilities|Time|GetGameTimeinSeconds) (+ (Variables|Default|GetLastTimeActivated) (Variables|Default|GetSwitchingCooldown)))))