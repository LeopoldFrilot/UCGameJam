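; BPC_MovementComponent is the player character component that handles jumping, double jumping and gravity tuning.
; It binds to the character's jump and landed events, zeroing vertical velocity and applying a separate jump power for air jumps, then restoring the base power on landing.
; Each tick it switches to a falling gravity scale while descending, unless a blocking action is active.
; Jump and double jump each post a Wwise sound.
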(event Custom|OnJump_Event
  (params (JumpCount :type Integer))
  (bind _character_movement_component (Variables|Default|GetCharacter%20Movement%20Component))
  (bind _returnvalue (Pawn|Components|CharacterMovement|GetLastUpdateVelocity _character_movement_component))
  (if (Character|CanJump (Variables|Default|GetCharacter))
    (Utilities|FlowControl|Sequence
      (:then_0
        (if (> JumpCount 0)
          (Variables|/Script/Engine.MovementComponent|SetVelocity _character_movement_component (Math|Vector|MakeVector (.x _returnvalue) (.y _returnvalue) 0.0))
          (Variables|/Script/Engine.CharacterMovementComponent|SetJumpZVelocity (Variables|Default|GetCharacter%20Movement%20Component) (Variables|Default|GetDoubleJumpPower))
          (Character|Jump (Variables|Default|GetCharacter))
          (else
            (Character|Jump (Variables|Default|GetCharacter)))))
      (:then_1
        ;[0.15 0.03339 0.1399 0.5] Wwise_Jump_DoubleJump
        (Utilities|FlowControl|Sequence
          (:then_0
            (if (== JumpCount 0)
              (Class|AkGameplayStatics|PostEvent "/Game/WwiseAudio/PlayerCharacter/Jump/player_jump.player_jump" (Components|GetOwner))))
          (:then_1
            (if (== JumpCount 1)
              (Class|AkGameplayStatics|PostEvent "/Game/WwiseAudio/PlayerCharacter/Jump/player_doublejump.player_doublejump" (Components|GetOwner)))))))))

(event Custom|OnCharacterLanded_Event
  (Variables|/Script/Engine.CharacterMovementComponent|SetJumpZVelocity (Variables|Default|GetCharacter%20Movement%20Component) (Variables|Default|GetBaseJumpPower)))

(event EventBeginPlay
  (bind _asbp_player_character (Utilities|Casting|CastToBP_PlayerCharacter (Components|GetOwner)))
  (Variables|Default|SetCharacter _asbp_player_character)
  (Variables|Default|SetCharacter%20Movement%20Component (Variables|/Script/Engine.Character|GetCharacterMovement _asbp_player_character))
  (EventDispatchers|AssignOnJump _asbp_player_character (delegate Custom|OnJump_Event))
  (EventDispatchers|AssignOnCharacterLanded _asbp_player_character (delegate Custom|OnCharacterLanded_Event)))

(event EventTick
  (params (DeltaSeconds :type Float%20%28single-precision%29))
  (CallFunction|UpdateGravity))

(fn UpdateGravity
  (bind _character_movement_component (Variables|Default|GetCharacter%20Movement%20Component))
  (if (not (Default|IsinBlockingAction (Variables|Default|GetCharacter)))
    (Variables|/Script/Engine.CharacterMovementComponent|SetGravityScale (Variables|Default|GetCharacter%20Movement%20Component) (Math|Float|SelectFloat (Variables|Default|GetFallingGravity) (Variables|Default|GetBaseGravity) (and (< (.z (Pawn|Components|CharacterMovement|GetLastUpdateVelocity _character_movement_component)) 0.0) (AI|Components|NavMovement|IsFalling _character_movement_component))))))