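; Base NPC actor that gives the player an ability on interaction, or queues post-puzzle dialogue through the game mode's dialogue runner if already unlocked.
; GetAbilityToGive and GetPostPuzzleDialogueID return empty defaults here.
; A half-second looping timer turns the sprite toward the player by flipping its X scale.
; The dialogue-finished handler bound to the child-actor dialogue player is empty, and the tangram puzzle widget creation is disconnected.
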(event Custom|CustomEvent
  (CallFunction|FacePlayer))

(event Custom|Interact
  (params (Player :type BP%20Player%20Character%20Object%20Reference))
  (bind _ability (CallFunction|GetAbilitytoGive))
  (bind _bpc_abilitymanager (Variables|/Game/Blueprints/Character/BP_PlayerCharacter.BP_PlayerCharacter_C|GetBPC_AbilityManager Player))
  (if (Utilities|Array|ContainsItem (Variables|/Game/Blueprints/Character/BPC_AbilityManager.BPC_AbilityManager_C|GetUnlockedAbilities _bpc_abilitymanager) _ability)
    (Default|TryQueueDialogue (Variables|/Game/Blueprints/Core/BP_GameMode.BP_GameMode_C|GetBPC_DialogueRunner (.AsBP%20Game%20Mode (Utilities|Casting|CastToBP_GameMode (Game|GetGameMode)))) (CallFunction|GetPostPuzzleDialogueID))
    (else
      (Default|UnlockAbility _bpc_abilitymanager _ability))))

(event Custom|DialogueFinished_Event)

(event EventBeginPlay
  (Utilities|Time|SetTimerbyEvent (delegate Custom|CustomEvent) 0.5 true)
  (bind _asbp_dialogue_player (Utilities|Casting|CastToBP_DialoguePlayer (Variables|/Script/Engine.ChildActorComponent|GetChildActor (Variables|Default|GetDialoguePlayer))))
  (EventDispatchers|AssignDialogueFinished _asbp_dialogue_player (delegate Custom|DialogueFinished_Event)))

(fn ConstructionScript)

(fn GetPostPuzzleDialogueID
  (return ""))

(fn GetAbilitytoGive
  (return 0))

(fn FacePlayer
  (bind _sprite (Variables|Default|GetSprite))
  (bind _relativescale3d (Variables|/Script/Engine.SceneComponent|GetRelativeScale3D _sprite))
  (Transformation|SetRelativeScale3D _sprite (Math|Vector|MakeVector (* (Math|Float|SelectFloat -1.0 1.0 (< (.x (Transformation|GetActorLocation (Game|Player|GetPlayerPawn 0))) (.x (Transformation|GetActorLocation)))) (Math|Float|Absolute(Float) (.x _relativescale3d))) (.y _relativescale3d) (.z _relativescale3d))))