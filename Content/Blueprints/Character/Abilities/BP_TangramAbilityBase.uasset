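; BP_TangramAbilityBase is the base actor for player character abilities, providing Activate, UpdatePassive and EndAbility events.
; Activate prints a debug message, then casts the actor's owner to BP_PlayerCharacter and caches it in PlayerCharacter.
; UpdatePassive only prints an active-status debug message, and EndAbility destroys the ability actor.
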(event Custom|Activate
  (Development|PrintString (Utilities|String|Append (Utilities|GetDisplayName self) " ACTIVATED"))
  (bind _asbp_player_character (Utilities|Casting|CastToBP_PlayerCharacter (Components|GetOwner)))
  (Variables|Default|SetPlayerCharacter _asbp_player_character))

(event Custom|UpdatePassive
  (Development|PrintString (Utilities|String|Append (Utilities|GetDisplayName self) " Active...") true false "(R=0.000000,G=0.380208,B=0.048626,A=1.000000)" 0.1 "ility"))

(event Custom|EndAbility
  (Actor|DestroyActor))

(fn ConstructionScript)