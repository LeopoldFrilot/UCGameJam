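; Bison character ability that makes the player dash left, right or straight down based on held direction.
; Activation zeroes gravity and velocity, applies a velocity-change impulse, plays Wwise charge sounds and starts a short timer to end the dash.
; EndDash clears the timer and momentum; when flagged as crashed, it launches the player upward with impact sounds.
; The dash sets gravity scale to zero but never restores it here.
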(event Custom|CustomEvent
  (CallFunction|EndDash false))

(event Custom|EndDash
  (params (Crashed :type Boolean))
  (bind _playercharacter (Variables|Default|GetPlayerCharacter))
  (bind _charactermovement (Variables|/Script/Engine.Character|GetCharacterMovement _playercharacter))
  (Variables|/Game/Blueprints/Character/BP_PlayerCharacter.BP_PlayerCharacter_C|SetIsPlayerDashing (Variables|Default|GetPlayerCharacter) false)
  (Utilities|Time|ClearandInvalidateTimerbyHandle (Variables|Default|GetDashTImer))
  (Pawn|Components|CharacterMovement|ClearAccumulatedForces (Variables|/Script/Engine.Character|GetCharacterMovement (Variables|Default|GetPlayerCharacter)))
  (Variables|/Script/Engine.MovementComponent|SetVelocity _charactermovement (Math|Vector|MakeVector 0.0 0.0 0.0))
  (if Crashed
    (Physics|AddImpulse _charactermovement "0.000000,0.000000,850.000000" true)
    (Class|AkGameplayStatics|PostEvent "/Game/WwiseAudio/_NewWwiseAssets/Animal/Bison/bison_gurgle.bison_gurgle" (Game|Player|GetPlayerPawn 0))
    (Class|AkGameplayStatics|PostEvent "/Game/WwiseAudio/_NewWwiseAssets/Actions/Actions/play_bison_impact.play_bison_impact" (Game|Player|GetPlayerPawn 0))))

(event EventActivate
  (bind _playercharacter (Variables|Default|GetPlayerCharacter))
  (bind _charactermovement (Variables|/Script/Engine.Character|GetCharacterMovement _playercharacter))
  (|CallParentFunction)
  (Utilities|FlowControl|Sequence
    (:then_0
      (Variables|/Game/Blueprints/Character/BP_PlayerCharacter.BP_PlayerCharacter_C|SetIsPlayerDashing (Variables|Default|GetPlayerCharacter) true)
      (Variables|/Script/Engine.CharacterMovementComponent|SetGravityScale _charactermovement 0.0)
      (Pawn|Components|CharacterMovement|ClearAccumulatedForces _charactermovement)
      (Variables|/Script/Engine.MovementComponent|SetVelocity _charactermovement (Math|Vector|MakeVector 0.0 0.0 0.0))
      (if (Utilities|Enum|Equal(Enum) (Variables|/Game/Blueprints/Character/BP_PlayerCharacter.BP_PlayerCharacter_C|GetHeldVerticalDirection (Variables|Default|GetPlayerCharacter)) "Down")
        (Physics|AddImpulse _charactermovement (Math|Vector|MakeVector 0.0 0.0 (* -1.0 (Variables|Default|GetDashStrength))) true)
        (else
          (Physics|AddImpulse _charactermovement (Math|Vector|MakeVector (* (Math|Float|SelectFloat -1.0 1.0 (Utilities|Enum|Equal(Enum) (Variables|/Game/Blueprints/Character/BP_PlayerCharacter.BP_PlayerCharacter_C|GetHeldHorizontalDirection (Variables|Default|GetPlayerCharacter)) "Left")) (Variables|Default|GetDashStrength)) 0.0 0.0) true))))
    (:then_1
      (bind _returnvalue (Utilities|Time|SetTimerbyEvent (delegate Custom|CustomEvent) 0.15))
      (Variables|Default|SetDashTImer _returnvalue)
      (Class|AkGameplayStatics|PostEvent "/Game/WwiseAudio/_NewWwiseAssets/Animal/Bison/bison_huff.bison_huff" (Game|Player|GetPlayerPawn 0))
      (Class|AkGameplayStatics|PostEvent "/Game/WwiseAudio/_NewWwiseAssets/Actions/Actions/play_bison_charge.play_bison_charge" (Game|Player|GetPlayerPawn 0)))))

(event EventEndAbility
  (CallFunction|EndDash false)
  (|CallParentFunction))

(fn ConstructionScript
  (|CallParentFunction))