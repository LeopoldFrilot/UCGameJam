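; Turtle ability Blueprint that gives the player a brief, timed parry window on activation.
; Activate sets the parrying flag on the player character and starts a short timer that closes the window, as does ending the ability.
; A Parry event clears accumulated forces and vertical velocity, launches the player upward with a mass-independent impulse, marks the damager as parried and closes the window.
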(event Custom|EndParryTimer
  (CallFunction|EndParry))

(event Custom|EndParry
  (Variables|/Game/Blueprints/Character/BP_PlayerCharacter.BP_PlayerCharacter_C|SetIsPlayerParrying (Variables|Default|GetPlayerCharacter) false)
  (Utilities|Time|ClearandInvalidateTimerbyHandle (Variables|Default|GetParryTImer)))

(event Custom|Parry
  (params (Damager :type BPI%20Damager%20Interface))
  (bind _playercharacter (Variables|Default|GetPlayerCharacter))
  (bind _charactermovement (Variables|/Script/Engine.Character|GetCharacterMovement _playercharacter))
  (Pawn|Components|CharacterMovement|ClearAccumulatedForces _charactermovement)
  (Variables|/Script/Engine.MovementComponent|SetVelocity _charactermovement (Math|Vector|MakeVector (.x (Variables|/Script/Engine.MovementComponent|GetVelocity _charactermovement)) (.y (Variables|/Script/Engine.MovementComponent|GetVelocity _charactermovement)) 0.0))
  (Physics|AddImpulse (Variables|/Script/Engine.Character|GetCharacterMovement (Variables|Default|GetPlayerCharacter)) "0.000000,0.000000,1200.000000" true)
  (Default|SetParried Damager)
  (CallFunction|EndParry))

(event EventBeginPlay)

(event Collision|EventActorBeginOverlap
  (params (OtherActor :type Actor%20Object%20Reference)))

(event EventTick
  (params (DeltaSeconds :type Float%20%28single-precision%29)))

(event EventActivate
  (|CallParentFunction)
  (Utilities|FlowControl|Sequence
    (:then_0
      (Variables|/Game/Blueprints/Character/BP_PlayerCharacter.BP_PlayerCharacter_C|SetIsPlayerParrying (Variables|Default|GetPlayerCharacter) true))
    (:then_1
      (bind _returnvalue (Utilities|Time|SetTimerbyEvent (delegate Custom|EndParryTimer) 0.2))
      (Variables|Default|SetParryTImer _returnvalue))))

(event EventEndAbility
  (CallFunction|EndParry)
  (|CallParentFunction))

(fn ConstructionScript
  (|CallParentFunction))