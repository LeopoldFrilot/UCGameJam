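; Player character component that plays grass footstep sounds through Wwise while the character moves.
; Move input above a small threshold fires a footstep through a DoOnce that a short fixed delay re-arms, setting the cadence.
; Footsteps are skipped while falling or when X velocity is zero.
; An alternative distance-based trigger, using ShouldResetDistanceTracker, remains in the graph but is disconnected.
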(event Custom|PlayFootstep
  (bind _returnvalue (Components|GetOwner))
  (bind _asbp_player_character (Utilities|Casting|CastToBP_PlayerCharacter _returnvalue))
  (if (not (AI|Components|NavMovement|IsFalling (Variables|/Script/Engine.Character|GetCharacterMovement _asbp_player_character)))
    (if (!= (.x (Variables|/Script/Engine.MovementComponent|GetVelocity (Pawn|GetMovementComponent _asbp_player_character))) 0.0)
      (Class|AkGameplayStatics|PostEvent "/Game/WwiseAudio/PlayerCharacter/Footsteps/player_footsteps_grass.player_footsteps_grass" _returnvalue))))

(event Input|EnhancedActionEvents|EnhancedInputActionIA_Move
  (params (ActionValue :type Vector%202D%20Structure) (ElapsedSeconds :type Float%20%28double-precision%29) (TriggeredSeconds :type Float%20%28double-precision%29) (InputAction :type Input%20Action%20Object%20Reference :default "/Game/Input/Actions/IA_Move.IA_Move"))
  (bind _output_get (Variables|Default|SetIsMoving (> (Math|Vector2D|Vector2DLength ActionValue) 0.1)))
  (if _output_get
    (Utilities|FlowControl|DoOnce false :!label _label
      (:Completed
        (CallFunction|PlayFootstep)
        (Utilities|FlowControl|Delay 0.235)
        (Class|TypedElementListLibrary|Reset)
        (goto _label Reset)))))

(event EventBeginPlay
  (Variables|Default|SetLastLocation (Transformation|GetActorLocation (Components|GetOwner))))

(event EventTick
  (params (DeltaSeconds :type Float%20%28single-precision%29)))

(fn ShouldResetDistanceTracker
  (bind _returnvalue (Components|GetOwner))
  (return (or (AI|Components|NavMovement|IsFalling (Actor|GetComponentbyClass _returnvalue "/Script/Engine.CharacterMovementComponent")) (Math|Vector|VectorIsNearlyZero (Transformation|GetVelocity _returnvalue)))))