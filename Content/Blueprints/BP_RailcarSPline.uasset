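; A railcar spline actor that moves a referenced actor along its Spline component.
; While not paused, Tick sets the rider's world location and rotation from the current spline distance, then advances that distance by RailcarSpeed scaled by delta time.
; Activate starts the ride from distance zero, while Reset pauses it, zeroes the distance and teleports the rider to this actor's location, where BeginPlay also places it.
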(event EventBeginPlay
  (Transformation|SetActorLocation (Variables|Default|GetActorRidingTheSpline) (Transformation|GetActorLocation) false true))

(event Collision|EventActorBeginOverlap
  (params (OtherActor :type Actor%20Object%20Reference)))

(event EventTick
  (params (DeltaSeconds :type Float%20%28single-precision%29))
  (bind _spline (Variables|Default|GetSpline))
  (if (not (Variables|Default|GetPaused))
    (Transformation|SetActorLocationAndRotation (Variables|Default|GetActorRidingTheSpline) (Spline|GetLocationatDistanceAlongSpline _spline (Variables|Default|GetPositionAlongSpline) "World") (Spline|GetRotationatDistanceAlongSpline _spline (Variables|Default|GetPositionAlongSpline) "World"))
    (Variables|Default|SetPositionAlongSpline (+ (Variables|Default|GetPositionAlongSpline) (* (Variables|Default|GetRailcarSpeed) (Utilities|Time|GetWorldDeltaSeconds))))))

(event EventActivate
  (Variables|Default|SetPaused false)
  (Variables|Default|SetPositionAlongSpline 0.0))

(event EventReset
  (params (NewLocation :type Vector :default "0, 0, 0"))
  (Variables|Default|SetPaused true)
  (Transformation|SetActorLocation (Variables|Default|GetActorRidingTheSpline) (Transformation|GetActorLocation) false true)
  (Variables|Default|SetPositionAlongSpline 0.0))

(fn ConstructionScript)