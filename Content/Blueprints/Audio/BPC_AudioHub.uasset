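; Audio hub component that shares one Wwise Ak component per audio event among multiple registered sources.
; The first registration spawns an auto-posting Ak component attached to the owner's root and maps it to the event with its source list.
; Later registrations only add the source.
; Unregistering a listed source removes it and stops the sound even if others remain, leaving the map entry in place.
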(event Custom|RegisterEventCOmponent
  (params (Event :type Ak%20Audio%20Event%20Object%20Reference) (Source :type Actor%20Object%20Reference))
  (bind _activeaudioevents (Variables|Default|GetActiveAudioEvents))
  (bind (_value _returnvalue) (Utilities|Map|Find _activeaudioevents Event))
  (Development|PrintString "+1")
  (if _returnvalue
    (Utilities|Array|AddUnique (.registeredsources _value) Source)
    (else
      (bind _returnvalue_2 (Class|AkGameplayStatics|SpawnAkComponentatLocation Event "0, 0, 0" "0, 0, 0" true true))
      (Transformation|AttachComponentToComponent _returnvalue_2 (Variables|/Script/Engine.Actor|GetRootComponent (Components|GetOwner)) "None" "SnapToTarget" "KeepRelative" "KeepRelative" true)
      (Utilities|Map|Add (Variables|Default|GetActiveAudioEvents) Event (Utilities|Struct|MakeF_ComponentList _returnvalue_2 (Utilities|Array|MakeArray Source))))))

(event Custom|UnRegisterComponent
  (params (Event :type Ak%20Audio%20Event%20Object%20Reference) (Source :type Actor%20Object%20Reference))
  (bind _activeaudioevents (Variables|Default|GetActiveAudioEvents))
  (bind (_value _returnvalue) (Utilities|Map|Find _activeaudioevents Event))
  (if _returnvalue
    (if (Utilities|Array|ContainsItem (.registeredsources _value) Source)
      (Development|PrintString "-1")
      (Utilities|Array|RemoveItem (.registeredsources _value) Source)
      (Class|AkGameObject|Stop (.spawn _value)))
    (else
      (Development|PrintString "Hello"))))

(event EventBeginPlay)

(event EventTick
  (params (DeltaSeconds :type Float%20%28single-precision%29)))