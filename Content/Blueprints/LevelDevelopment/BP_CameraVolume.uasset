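; Camera volume that confines the player's camera boom to a bounded area while the character is inside it.
; Entering the Outer box attaches the boom to the Inner box, which follows the character each tick.
; Inner is clamped by both box extents to stay within Outer on X and Z, while Y follows freely.
; Exiting reattaches the boom to the character's capsule and restores both boxes to their starting locations.
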(event OnComponentBeginOverlap(Outer)
  (params (OverlappedComponent :type Primitive%20Component%20Object%20Reference) (OtherActor :type Actor%20Object%20Reference) (OtherComp :type Primitive%20Component%20Object%20Reference) (OtherBodyIndex :type Integer) (bFromSweep :type Boolean) (SweepResult :type Hit%20Result%20Structure%20%28by%20ref%29))
  (bind _asbp_player_character (Utilities|Casting|CastToBP_PlayerCharacter OtherActor))
  (Variables|Default|SetFollowCharacter _asbp_player_character)
  (Transformation|AttachComponentToComponent (Variables|/Game/Blueprints/Character/BP_PlayerCharacter.BP_PlayerCharacter_C|GetCameraBoom _asbp_player_character) (Variables|Default|GetInner) "None" "SnapToTarget" "KeepRelative" "KeepRelative" true))

(event OnComponentEndOverlap(Outer)
  (params (OverlappedComponent :type Primitive%20Component%20Object%20Reference) (OtherActor :type Actor%20Object%20Reference) (OtherComp :type Primitive%20Component%20Object%20Reference) (OtherBodyIndex :type Integer))
  (bind _asbp_player_character (Utilities|Casting|CastToBP_PlayerCharacter OtherActor))
  (Variables|Default|SetFollowCharacter 0)
  (Transformation|AttachComponentToComponent (Variables|/Game/Blueprints/Character/BP_PlayerCharacter.BP_PlayerCharacter_C|GetCameraBoom _asbp_player_character) (Variables|/Script/Engine.Character|GetCapsuleComponent _asbp_player_character) "None" "SnapToTarget" "KeepRelative" "KeepRelative" true)
  (Transformation|SetWorldLocation (Variables|Default|GetOuter) (Variables|Default|GetOuterRootLocation) false true)
  (Transformation|SetWorldLocation (Variables|Default|GetInner) (Variables|Default|GetInnerRootLocation) false true))

(event EventBeginPlay
  (Variables|Default|SetInnerRootLocation (Transformation|GetWorldLocation (Variables|Default|GetInner)))
  (Variables|Default|SetOuterRootLocation (Transformation|GetWorldLocation (Variables|Default|GetOuter))))

(event EventTick
  (params (DeltaSeconds :type Float%20%28single-precision%29))
  (bind _followcharacter (Variables|Default|GetFollowCharacter)
    (:then
      (CallFunction|ClampedMoveInner (Transformation|GetActorLocation _followcharacter)))
    (:else)))

(fn ConstructionScript)

(fn ClampedMoveInner
  (params (TargetLocation :type Vector))
  (bind _inner (Variables|Default|GetInner))
  (bind _outer (Variables|Default|GetOuter))
  (bind _inner_2 (Variables|Default|GetInner))
  (bind _returnvalue (Components|Box|GetScaledBoxExtent _outer))
  (bind _returnvalue_2 (Transformation|GetWorldLocation _outer))
  (bind _returnvalue_3 (Components|Box|GetScaledBoxExtent _inner_2))
  (bind _returnvalue_4 (Components|Box|GetScaledBoxExtent _inner))
  (Transformation|SetWorldLocation (Variables|Default|GetInner) (Math|Vector|MakeVector (Math|Float|Clamp(Float) (.x TargetLocation) (+ (.x _returnvalue_3) (- (.x _returnvalue_2) (.x _returnvalue))) (- (+ (.x _returnvalue_2) (.x _returnvalue)) (.x _returnvalue_3))) (.y TargetLocation) (Math|Float|Clamp(Float) (.z TargetLocation) (+ (- (.z _returnvalue_2) (.z _returnvalue)) (.z _returnvalue_4)) (- (+ (.z _returnvalue_2) (.z _returnvalue)) (.z _returnvalue_4)))) false false))