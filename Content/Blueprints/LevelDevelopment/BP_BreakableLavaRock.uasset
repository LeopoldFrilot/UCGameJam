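; BP_BreakableLavaRock is a lava rock hazard that kills the player unless they are dashing when it tries to kill them.
; TryKillPlayer checks the player's dash state, either calling KillPlayer or setting TriedKilling, which blocks further kill attempts.
; Reset runs the parent's reset and clears that flag, while both parry queries return false.
; No breaking logic appears in this Blueprint itself.
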(event EventBeginPlay
  (|CallParentFunction) ; This node is disabled and will not be called.\nDrag off pins to build functionality.
)

(event Collision|EventActorBeginOverlap
  (params (OtherActor :type Actor%20Object%20Reference))
  (|CallParentFunction OtherActor) ; This node is disabled and will not be called.\nDrag off pins to build functionality.
)

(event EventTick
  (params (DeltaSeconds :type Float%20%28single-precision%29))
  (|CallParentFunction DeltaSeconds) ; This node is disabled and will not be called.\nDrag off pins to build functionality.
)

(event EventTryKillPlayer
  (if (not (Variables|Default|GetTriedKilling))
    (bind _asbp_player_character (Utilities|Casting|CastToBP_PlayerCharacter (Game|Player|GetPlayerPawn 0)))
    (if (Variables|/Game/Blueprints/Character/BP_PlayerCharacter.BP_PlayerCharacter_C|GetIsPlayerDashing _asbp_player_character)
      (Variables|Default|SetTriedKilling true)
      (else
        (Default|KillPlayer _asbp_player_character)))))

(event EventReset
  (params (NewLocation :type Vector :default "0, 0, 0"))
  (|CallParentFunction NewLocation)
  (Variables|Default|SetTriedKilling false))

(fn ConstructionScript
  (|CallParentFunction))

(fn IsParried
  (return false))

(fn IsParryable
  (return false))