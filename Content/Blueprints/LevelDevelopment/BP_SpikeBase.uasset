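; BP_SpikeBase is a base spike hazard that can kill the player and be parried.
; TryKillPlayer casts player pawn 0 to BP_PlayerCharacter and calls KillPlayer, without checking the parried state.
; SetParried and Reset toggle a Parried flag exposed through IsParried, and IsParryable always returns true.
; The base has no active overlap or tick logic and never calls TryKillPlayer itself.
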(event EventBeginPlay)

(event Collision|EventActorBeginOverlap
  (params (OtherActor :type Actor%20Object%20Reference)))

(event EventTick
  (params (DeltaSeconds :type Float%20%28single-precision%29)))

(event EventSetParried
  (Variables|Default|SetParried true))

(event EventReset
  (params (NewLocation :type Vector :default "0, 0, 0"))
  (Variables|Default|SetParried false))

(event EventTryKillPlayer
  (bind _asbp_player_character (Utilities|Casting|CastToBP_PlayerCharacter (Game|Player|GetPlayerPawn 0)))
  (Default|KillPlayer _asbp_player_character))

(fn ConstructionScript)

(fn IsParried
  (return (Variables|Default|GetParried)))

(fn IsParryable
  (return true))