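; BP_BreakableActor is a level actor that can be broken and restored through Break and Reset events.
; Break sets the Broken flag, hides the StaticMesh with visibility propagated to children, and disables collision on it and its child static mesh components.
; Reset clears the flag, shows the meshes again and sets their collision to query and physics.
; Nothing in this Blueprint calls either event.
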(event Custom|Break
  (bind _staticmesh (Variables|Default|GetStaticMesh))
  (Variables|Default|SetBroken true)
  (Rendering|SetVisibility _staticmesh false true)
  (Collision|SetCollisionEnabled _staticmesh "NoCollision")
  (for _array_element (Components|GetChildrenComponents _staticmesh false)
    (bind _asstatic_mesh_component (Utilities|Casting|CastToStaticMeshComponent _array_element))
    (Collision|SetCollisionEnabled _asstatic_mesh_component "NoCollision")))

(event EventBeginPlay)

(event Collision|EventActorBeginOverlap
  (params (OtherActor :type Actor%20Object%20Reference)))

(event EventTick
  (params (DeltaSeconds :type Float%20%28single-precision%29)))

(event EventReset
  (params (NewLocation :type Vector :default "0, 0, 0"))
  (bind _staticmesh (Variables|Default|GetStaticMesh))
  (Variables|Default|SetBroken false)
  (Rendering|SetVisibility _staticmesh true true)
  (Collision|SetCollisionEnabled _staticmesh "QueryAndPhysics")
  (for _array_element (Components|GetChildrenComponents _staticmesh false)
    (bind _asstatic_mesh_component (Utilities|Casting|CastToStaticMeshComponent _array_element))
    (Collision|SetCollisionEnabled _asstatic_mesh_component "QueryAndPhysics")))

(fn ConstructionScript)