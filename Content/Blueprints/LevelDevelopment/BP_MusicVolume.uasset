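; BP_MusicVolume is a box trigger volume that switches a set of audio loops on and off as the player enters and leaves it.
; Overlaps register or unregister each loop with the player character's BPCAudioHub, using the volume as source and a Playing flag against repeat starts.
; A delayed BeginPlay check catches players already inside.
; CheckBlocked tests required or blocking abilities, but the shown graphs never call it.
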(event OnComponentBeginOverlap(Box)
  (params (OverlappedComponent :type Primitive%20Component%20Object%20Reference) (OtherActor :type Actor%20Object%20Reference) (OtherComp :type Primitive%20Component%20Object%20Reference) (OtherBodyIndex :type Integer) (bFromSweep :type Boolean) (SweepResult :type Hit%20Result%20Structure%20%28by%20ref%29))
  (CallFunction|StartOverlapforPlayer OtherActor))

(event OnComponentEndOverlap(Box)
  (params (OverlappedComponent :type Primitive%20Component%20Object%20Reference) (OtherActor :type Actor%20Object%20Reference) (OtherComp :type Primitive%20Component%20Object%20Reference) (OtherBodyIndex :type Integer))
  (bind _asbp_player_character (Utilities|Casting|CastToBP_PlayerCharacter OtherActor))
  (Variables|Default|SetPlaying false)
  (for _array_element (Variables|Default|GetAudioLoopsToPlay)
    (Default|UnRegisterComponent (Variables|/Game/Blueprints/Character/BP_PlayerCharacter.BP_PlayerCharacter_C|GetBPC_AudioHub _asbp_player_character) _array_element self)))

(event EventBeginPlay
  (bind _returnvalue (Game|Player|GetPlayerPawn 0))
  (Utilities|FlowControl|Delay 0.2)
  (if (Collision|IsOverlappingActor (Variables|Default|GetBox) _returnvalue :!class /Script/Engine.PrimitiveComponent)
    (CallFunction|StartOverlapforPlayer _returnvalue)))

(event EventTick
  (params (DeltaSeconds :type Float%20%28single-precision%29)))

(fn ConstructionScript)

(fn StartOverlapforPlayer
  (params (Object :type Object%20Object%20Reference))
  (bind _asbp_player_character (Utilities|Casting|CastToBP_PlayerCharacter Object))
  (if (not (Variables|Default|GetPlaying))
    (Variables|Default|SetPlaying true)
    (for _array_element (Variables|Default|GetAudioLoopsToPlay)
      (Default|RegisterEventCOmponent (Variables|/Game/Blueprints/Character/BP_PlayerCharacter.BP_PlayerCharacter_C|GetBPC_AudioHub _asbp_player_character) _array_element self))))

(fn CheckBlocked
  (params (Player :type BP%20Player%20Character%20Object%20Reference))
  (bind _bpc_abilitymanager (Variables|/Game/Blueprints/Character/BP_PlayerCharacter.BP_PlayerCharacter_C|GetBPC_AbilityManager Player))
  (bind _blockedability (Variables|Default|GetBlockedAbility))
  (bind _requiredability (Variables|Default|GetRequiredAbility))
  (bind _unlockedabilities (Variables|/Game/Blueprints/Character/BPC_AbilityManager.BPC_AbilityManager_C|GetUnlockedAbilities _bpc_abilitymanager))
  (if (and (Utilities|IsValidClass _blockedability) (Utilities|Array|ContainsItem _unlockedabilities _blockedability))
    (return true)
    (elif (Utilities|IsValidClass _requiredability)
      (return (not (Utilities|Array|ContainsItem _unlockedabilities _requiredability)))
      (else
        (return false)))))